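; BP_Garlic is a physics-driven garlic actor that kills enemies it strikes at speed.
; On a hit, it calls KillFunny on a BP_Enemy if the static mesh's linear velocity exceeds a threshold.
; Tick runs through a short Delay to periodically check for near-zero velocity, then spawns a disappearance effect and destroys the actor once it has come to rest.
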(event EventBeginPlay)

(event Collision|EventActorBeginOverlap
  (params (OtherActor :type Actor%20Object%20Reference)))

(event EventTick
  (params (DeltaSeconds :type Float%20%28single-precision%29))
  (Utilities|FlowControl|Delay 0.2)
  (if (Utilities|Operators|EqualEqual :A (Transformation|GetVelocity) :ErrorTolerance 1e+01)
    (Niagara|SpawnSystematLocation "/Game/FX/FX_GarlicDisappearance.FX_GarlicDisappearance" (Transformation|GetActorLocation))
    (Actor|DestroyActor)))

(event Collision|EventHit
  (params (MyComp :type Primitive%20Component%20Object%20Reference) (Other :type Actor%20Object%20Reference) (OtherComp :type Primitive%20Component%20Object%20Reference) (bSelfMoved :type Boolean) (HitLocation :type Vector :default "0, 0, 0") (HitNormal :type Vector :default "0, 0, 0") (NormalImpulse :type Vector :default "0, 0, 0") (Hit :type Hit%20Result%20Structure%20%28by%20ref%29))
  (bind _asbp_enemy (Utilities|Casting|CastToBP_Enemy (Components|GetOwner OtherComp)))
  (bind _returnvalue (Physics|GetPhysicsLinearVelocity (Variables|Debug|GetStaticMeshComponent) "None"))
  (if (> (Math|Vector|VectorLength _returnvalue) 1e+02)
    (Default|KillFunny _asbp_enemy)))

(fn ConstructionScript)