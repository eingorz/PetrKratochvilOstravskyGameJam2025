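; Enemy character that wanders to random reachable points on a looping timer until PawnSensing spots a pawn, then permanently pauses wandering and runs at the player.
; On reaching the player it triggers an AnimBP attack, then damages and launches them if still close after a delay; attacking re-arms only after a hit.
; Damage updates a distance-shown health bar widget and leads to an animated death, with a separate blood-splat instant kill.
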(event OnSeePawn(PawnSensing)
  (params (Pawn :type Pawn%20Object%20Reference))
  ;[0.15 0.15 0.15 0.5] Sense player and call player
  (Variables|Default|SetPlayerNoticed true)
  (Utilities|Time|PauseTimerbyHandle (Variables|Default|GetWanderingTimerHandle))
  (CallFunction|FollowPlayer))

(event Custom|FollowPlayer
  (bind _returnvalue (Game|Player|GetPlayerPawn 0))
  (bind _capsulecomponent (Variables|Collision|GetCapsuleComponent))
  (bind _returnvalue_2 (Math|Vector|GetForwardVector _capsulecomponent))
  (bind _returnvalue_3 (* _returnvalue_2 6e+02))
  ;[0.15 0.15 0.15 0.5] Find and Attacks finder if found
  (if (Variables|Default|GetPlayerNoticed)
    (Variables|/Script/Engine.CharacterMovementComponent|SetMaxWalkSpeed (Variables|Character|GetCharacterMovement self) 6e+02)
    (AI|AIMoveTo self "0, 0, 0" _returnvalue 5e+01 false
      (:OnSuccess
        (if (Variables|Default|GetcanAttack)
          (Variables|Default|SetcanAttack false)
          (bind _asbp_first_person_character (Utilities|Casting|CastToBP_FirstPersonCharacter _returnvalue))
          (bind _asap_enemy_ap (Utilities|Casting|CastToAP_EnemyAP (Components|SkeletalMesh|GetAnimInstance (Variables|Character|GetMesh))))
          (Variables|/Game/Enemy/AP_EnemyAP.AP_EnemyAP_C|SetAttack _asap_enemy_ap true)
          (Utilities|FlowControl|Delay 0.73)
          (if (< (Math|Vector|Distance(Vector) (Transformation|GetActorLocation _asbp_first_person_character) (Transformation|GetActorLocation)) 2.6e+02)
            (Default|TakeDamage _asbp_first_person_character (Variables|Default|GetHitDamage))
            (Character|LaunchCharacter _asbp_first_person_character (Math|Vector|MakeVector (.x _returnvalue_3) (.y _returnvalue_3) 2e+02) false false)
            (Utilities|FlowControl|Delay 0.73)
            (Variables|/Game/Enemy/AP_EnemyAP.AP_EnemyAP_C|SetAttack _asap_enemy_ap false)
            (Variables|Default|SetcanAttack true)))))))

(event Custom|WanderEvent
  (bind _self self)
  ;[0.15 0.15 0.15 0.5] Create Wander timer, get rand location and move guy there
  (Variables|/Script/Engine.CharacterMovementComponent|SetMaxWalkSpeed (Variables|Character|GetCharacterMovement _self) 3e+02)
  (AI|AIMoveTo _self (.RandomLocation (AI|Navigation|GetRandomReachablePointinRadius (Transformation|GetActorLocation) 5e+03 0 0)) 0 2e+02 false))

(event Custom|EnemyTakeDamage
  (params (DamageAmount :type Integer))
  ;[0.15 0.15 0.15 0.5] Take Damage, Kill if dead
  (bind _output_get (Variables|Default|SetEnemyHP (- (Variables|Default|GetEnemyHP) DamageAmount)))
  (Default|UpdateHealth (Variables|Default|GetAs%20UWG%20Enemyhealth) _output_get)
  (if (<= _output_get 0)
    (CallFunction|KIllNormal)))

(event Custom|KillFunny
  (bind _returnvalue (Transformation|GetActorLocation))
  (Audio|PlaySoundatLocation "/Game/Sounds/splat_sound_effects__no_copyright_.splat_sound_effects__no_copyright_" _returnvalue "0, 0, 0" 1.0 1.0 0.0 0 0 0 0)
  (Niagara|SpawnSystematLocation "/Game/FX/FX_BloodSplat.FX_BloodSplat" _returnvalue)
  (Actor|DestroyActor))

(event Custom|KIllNormal
  (Pawn|Components|CharacterMovement|DisableMovement (Variables|Character|GetCharacterMovement))
  (bind _asap_enemy_ap (Utilities|Casting|CastToAP_EnemyAP (Components|SkeletalMesh|GetAnimInstance (Variables|Character|GetMesh))))
  (Variables|/Game/Enemy/AP_EnemyAP.AP_EnemyAP_C|SetDying _asap_enemy_ap true)
  (Utilities|FlowControl|Delay (Animation|GetPlayLength (Variables|Default|GetDeathAnim)))
  (Actor|DestroyActor))

(event EventBeginPlay
  (bind _asuwg_enemyhealth (Utilities|Casting|CastToUWG_Enemyhealth (UserInterface|GetWidget (Variables|Default|GetHealthBar))))
  (Variables|Default|SetAs%20UWG%20Enemyhealth _asuwg_enemyhealth)
  ;[0.15 0.15 0.15 0.5] Create Wander timer, get rand location and move guy there
  (bind _returnvalue (Utilities|Time|SetTimerbyEvent (delegate Custom|WanderEvent) 2.0 true))
  (Variables|Default|SetWanderingTimerHandle _returnvalue))

(event Collision|EventActorBeginOverlap
  (params (OtherActor :type Actor%20Object%20Reference)))

(event EventTick
  (params (DeltaSeconds :type Float%20%28single-precision%29))
  (if (> (Variables|Default|GetHealthBarViewDistance) (Transformation|GetDistanceTo (Game|GetPlayerCharacter 0) self))
    (Rendering|SetVisibility (Variables|Default|GetHealthBar) true false)
    (else
      (Rendering|SetVisibility (Variables|Default|GetHealthBar) false false))))

(fn ConstructionScript)